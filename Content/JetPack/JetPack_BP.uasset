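; Jetpack actor that shows thruster effects while its parent third-person character is in jetpack mode.
; Each Tick it casts its parent actor to BP_ThirdPersonCharacter and reads JetPackMode to set the visibility of the left and right thruster effects.
; It only handles this visual toggle and contains no flight or input logic.
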(event `self.ReceiveTick`
  (params (DeltaSeconds :type "Float (single-precision)"))
  (bind _asbp_third_person_character (cast `/Game/ThirdPerson/Blueprints/BP_ThirdPersonCharacter` (`self.GetParentActor`)))
  (if (`/Game/ThirdPerson/Blueprints/BP_ThirdPersonCharacter.JetPack Mode` _asbp_third_person_character)
    (`SceneComponent.SetVisibility` (`self.ThrusterEffect_L`) true false)
    (`SceneComponent.SetVisibility` (`self.ThrusterEffect_R`) true false)
    (else
      (`SceneComponent.SetVisibility` (`self.ThrusterEffect_L`) false false)
      (`SceneComponent.SetVisibility` (`self.ThrusterEffect_R`) false false))))

(fn `UserConstructionScript`)